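; BP_WitnessTiles is a board tile in the LoopHero game that triggers the Witness NPC's dialogue.
; On BeginPlay it runs the parent logic, then finds and caches the BP_Witness actor in the level.
; When ActivateTiles fires, it checks that the cached NPC is valid, opens its dialogue and sets a flag to true on the game instance.
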(event `self.ReceiveBeginPlay`
  (`parent.ReceiveBeginPlay`)
  (`|ExecutionSequence`
    (:`then_0`
      (bind _returnvalue (`GameplayStatics.GetActorOfClass` "/Game/LoopHero/BP_Witness.BP_Witness_C"))
      (set `self.NPCWitness` _returnvalue))))

(event `self.ActivateTiles`
  (bind _npcwitness (`self.NPCWitness`))
  (if (`KismetSystemLibrary.IsValid` _npcwitness)
    (`/Game/LoopHero/BP_Witness.OpenDialogue` _npcwitness)
    (`/Game/LoopHero/BP_GI_LoopHero.DefineFlag` (`self.Gameinstance`) "NewEnumerator0" true)))

(fn `UserConstructionScript`
  (`parent.UserConstructionScript`))