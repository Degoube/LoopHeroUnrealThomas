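; BP_TilesAutel is an altar board tile that reports the altar's state when activated.
; ActivateTiles reads two GameInstance flags, the first gating on what appears to be the relic and the second on whether the altar is already active.
; It prints one of three French messages for inactive, lighting up or already active.
; The event only displays text and never sets either flag.
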(event `self.ActivateTiles`
  (bind _gameinstance (`self.Gameinstance`))
  (bind _value (`/Game/LoopHero/BP_GI_LoopHero.GetFlag` _gameinstance "NewEnumerator2"))
  (if _value
    (bind _value_2 (`/Game/LoopHero/BP_GI_LoopHero.GetFlag` _gameinstance "NewEnumerator3"))
    (if (not _value_2)
      (`KismetSystemLibrary.PrintString` "L'autel s'illumine avec la relique!" true true (struct :`G` 0.66 :`B` 1.0 :`A` 1.0) 5.0)
      (else
        (`KismetSystemLibrary.PrintString` "L'autel est déjà actif." true true (struct :`G` 0.66 :`B` 1.0 :`A` 1.0) 5.0)))
    (else
      (`KismetSystemLibrary.PrintString` "Un autel inactif. Il manque quelque chose..." true true (struct :`G` 0.66 :`B` 1.0 :`A` 1.0) 5.0))))

(fn `UserConstructionScript`
  (`parent.UserConstructionScript`))