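; BP_TilesCombat is a combat tile on the LoopHero board that resolves a simulated fight as a coin flip when activated.
; ActivateTiles rolls a random float, prints a French win or loss message, and adds or removes a fixed amount of resources through the game instance.
; It has no other logic: BeginPlay, Tick and overlap are disabled stubs, and the construction script only calls its parent.
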(event `self.ActivateTiles`
  (bind _gameinstance (`self.Gameinstance`))
  (if (> (`KismetMathLibrary.RandomFloatInRange` 0.0 1.0) 0.5)
    (`KismetSystemLibrary.PrintString` "Combat! Vous gagnez" true true (struct :`G` 0.66 :`B` 1.0 :`A` 1.0) 5.0)
    (`/Game/LoopHero/BP_GI_LoopHero.AddRessources` _gameinstance 20)
    (else
      (`KismetSystemLibrary.PrintString` "Combat! Vous perdez" true true (struct :`G` 0.66 :`B` 1.0 :`A` 1.0) 5.0)
      (`/Game/LoopHero/BP_GI_LoopHero.RemoveResources` _gameinstance 20))))

(fn `UserConstructionScript`
  (`parent.UserConstructionScript`))