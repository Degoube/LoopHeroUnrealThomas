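; BP_RuinsTiles is a ruins board tile for the LoopHero game that shows exploration text when activated.
; Its ActivateTiles event checks a Game Instance flag to tell whether the ruins were already explored.
; The first activation prints a French discovery message and sets the flag, while later activations print an already-explored message.
; Feedback uses only PrintString, and the flag is a fixed enum entry, so it is not tracked per tile.
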(event `self.ActivateTiles`
  (bind _gameinstance (`self.Gameinstance`))
  (bind _value (`/Game/LoopHero/BP_GI_LoopHero.GetFlag` _gameinstance "NewEnumerator1"))
  (if (not _value)
    (`KismetSystemLibrary.PrintString` "Des ruines anciennes... Des symboles étranges." true true (struct :`G` 0.66 :`B` 1.0 :`A` 1.0) 5.0)
    (`/Game/LoopHero/BP_GI_LoopHero.DefineFlag` _gameinstance "NewEnumerator1" true)
    (else
      (`KismetSystemLibrary.PrintString` "Vous avez déjà exploré ces ruines." true true (struct :`G` 0.66 :`B` 1.0 :`A` 1.0) 5.0))))

(fn `UserConstructionScript`
  (`parent.UserConstructionScript`))