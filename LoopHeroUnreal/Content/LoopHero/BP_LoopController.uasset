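; Loop controller for a dice-driven board loop: it builds a ring of tiles and moves the player around it.
; BeginPlay caches references, creates the HUD, then spawns six tile types on a circle using cos/sin after a delay.
; RollDice shows a 1-6 result and triggers MovePlayer, which steps through tiles and calls ActivateTiles.
; CheckLoopEnd increments the GameInstance loop counter at the last tile and resets the player to the first.
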(event `self.ReceiveBeginPlay`
  (bind _radius (`self.Radius`))
  (`|ExecutionSequence`
    (:`then_0`
      (bind _asbp_gi_loop_hero (cast `/Game/LoopHero/BP_GI_LoopHero` (`GameplayStatics.GetGameInstance`)))
      (set `self.GameInstance` _asbp_gi_loop_hero))
    (:`then_1`
      (bind _asbp_gm_loop_hero (cast `/Game/LoopHero/BP_GM_LoopHero` (`GameplayStatics.GetGameMode`)))
      (set `self.As BP GM Loop Hero` _asbp_gm_loop_hero))
    (:`then_2`
      (bind _returnvalue (`GameplayStatics.GetActorOfClass` "/Game/LoopHero/BP_Player.BP_Player_C"))
      (set `self.Player` _returnvalue))
    (:`then_3`
      (bind _returnvalue_2 (`|CreateWidget` "/Game/LoopHero/UI/WBP_HUD.WBP_HUD_C" (`GameplayStatics.GetPlayerController` 0)))
      (set `self.WBPHUD` _returnvalue_2))
    (:`then_4`
      (`KismetSystemLibrary.Delay` 1.0)
      (for _index (range 6)
        (switch `int` _index
          (:`0`
            (bind _returnvalue_3 (`KismetMathLibrary.DegreesToRadians` (* (/ _index (`self.LoopLenght`)) 360.0)))
            (bind _returnvalue_4 (`KismetMathLibrary.Conv_VectorToTransform` (`KismetMathLibrary.MakeVector` (* (`KismetMathLibrary.Cos` _returnvalue_3) _radius) (* (`KismetMathLibrary.Sin` _returnvalue_3) _radius) (`self.TilesHeight`))))
            (bind _returnvalue_5 (`|SpawnActorFromClass` "/Game/LoopHero/Board/BP_WitnessTiles.BP_WitnessTiles_C" _returnvalue_4 "Undefined" "MultiplyWithRoot" null null))
            (`KismetArrayLibrary.Array_Add` (`self.Tiles`) _returnvalue_5))
          (:`1`
            (bind _returnvalue_6 (`|SpawnActorFromClass` "/Game/LoopHero/Board/BP_TilesCombat.BP_TilesCombat_C" _returnvalue_4 "Undefined" "MultiplyWithRoot" null null))
            (`KismetArrayLibrary.Array_Add` (`self.Tiles`) _returnvalue_6))
          (:`2`
            (bind _returnvalue_7 (`|SpawnActorFromClass` "/Game/LoopHero/Board/BP_TilesRelic.BP_TilesRelic_C" _returnvalue_4 "Undefined" "MultiplyWithRoot" null null))
            (`KismetArrayLibrary.Array_Add` (`self.Tiles`) _returnvalue_7))
          (:`3`
            (bind _returnvalue_8 (`|SpawnActorFromClass` "/Game/LoopHero/Board/BP_TilesAutel.BP_TilesAutel_C" _returnvalue_4 "Undefined" "MultiplyWithRoot" null null))
            (`KismetArrayLibrary.Array_Add` (`self.Tiles`) _returnvalue_8))
          (:`4`
            (bind _returnvalue_9 (`|SpawnActorFromClass` "/Game/LoopHero/Board/BP_RuinsTiles.BP_RuinsTiles_C" _returnvalue_4 "Undefined" "MultiplyWithRoot" null null))
            (`KismetArrayLibrary.Array_Add` (`self.Tiles`) _returnvalue_9))
          (:`5`
            (bind _returnvalue_10 (`|SpawnActorFromClass` "/Game/LoopHero/Board/BP_Tiles.BP_Tiles_C" _returnvalue_4 "Undefined" "MultiplyWithRoot" null null))
            (`KismetArrayLibrary.Array_Add` (`self.Tiles`) _returnvalue_10)))
        (set `self.CurrentPosition` 0)
        (`self.K2_SetActorLocation` (`self.Player`) (+ (`self.K2_GetActorLocation` (`|GetArrayItem` (`self.Tiles`))) (0.0 0.0 50.0)) false true)))))

(event `RollDice`
  (bind _output_get (set `self.DiceResult` (`KismetMathLibrary.RandomIntegerInRange` 1 6)))
  (`/Game/LoopHero/UI/WBP_HUD.ShowDiceResult` (`self.WBPHUD`) _output_get)
  (`self.MovePlayer`))

(event `MovePlayer`
  (for _ (range (`self.DiceResult`))
    (bind _output_get (set `self.CurrentPosition` (mod (+ (`self.CurrentPosition`) 1) (`self.LoopLenght`))))
    (bind _output (`|GetArrayItem` (`self.Tiles`) _output_get))
    (`self.K2_SetActorLocation` (`self.Player`) (+ (`self.K2_GetActorLocation` _output) (0.0 0.0 50.0)) true false)
    (`KismetSystemLibrary.Delay` 0.2)
    (`/Game/LoopHero/Board/BP_Tiles.ActivateTiles` _output)
    (`self.CheckLoopEnd`)))

(fn `CheckLoopEnd`
  (if (== (`self.CurrentPosition`) (- (`self.LoopLenght`) 1))
    (`/Engine/EditorBlueprintResources/StandardMacros.IncrementInt` (`.LoopCounter_9_634EFF7C43FBCF3EED654895694C44E1` (break `/Game/LoopHero/Structure/S_NarrativeState` (`/Game/LoopHero/BP_GI_LoopHero.NarrativeState` (`self.GameInstance`))))
      (:`  `
        (bind _output_get (set `self.CurrentPosition` 0))
        (`self.K2_SetActorLocation` (`self.Player`) (`self.K2_GetActorLocation` (`|GetArrayItem` (`self.Tiles`) _output_get)) false false)
        (return)))
    (else
      (return))))

(fn `UserConstructionScript`)