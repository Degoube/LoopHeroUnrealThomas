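; Game mode for LoopHero that loads saved progress, shows the HUD and watches for the end of the game.
; On BeginPlay it caches the game instance, calls LoadProgress and creates WBP_HUD after a short delay.
; A looping timer, started a few seconds later, polls a win flag and a low-resource threshold on the game instance, adding the win or defeat screen whenever either condition holds.
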(event `self.ReceiveBeginPlay`
  (bind _returnvalue (`GameplayStatics.GetGameInstance`))
  (`|ExecutionSequence`
    (:`then_0`
      (`/Engine/EditorBlueprintResources/StandardMacros.IsValid` _returnvalue
        (:`Is Valid`
          (bind _asbp_gi_loop_hero (cast `/Game/LoopHero/BP_GI_LoopHero` _returnvalue))
          (bind _output_get (set `self.GameInstance` _asbp_gi_loop_hero))
          (`KismetSystemLibrary.PrintString` "Hello")
          (`/Game/LoopHero/BP_GI_LoopHero.LoadProgress` _output_get))))
    (:`then_1`
      (`KismetSystemLibrary.Delay` 0.1)
      (bind _returnvalue_2 (`|CreateWidget` "/Game/LoopHero/UI/WBP_HUD.WBP_HUD_C" (`GameplayStatics.GetPlayerController` 0)))
      (bind _output_get_2 (set `self.HUD` _returnvalue_2))
      (`UserWidget.AddToViewport` _output_get_2 0))
    (:`then_2`
      (`KismetSystemLibrary.Delay` 3.0)
      (`KismetSystemLibrary.K2_SetTimerDelegate` (delegate `CheckCondition`) 0.1 true))))

(event `CheckCondition`
  (`self.CheckWinCondition`)
  (`self.CheckLoseCondition`))

(fn `CheckLoseCondition`
  (bind (_narrativestate_flags _narrativestate_loopcounter _narrativestate_ressource) (break `/Game/LoopHero/Structure/S_NarrativeState` (`/Game/LoopHero/BP_GI_LoopHero.NarrativeState` (`self.GameInstance`))))
  (if (< _narrativestate_ressource 5)
    (bind _returnvalue (`|CreateWidget` "/Game/LoopHero/UI/WBP_DefeatScreen.WBP_DefeatScreen_C"))
    (`UserWidget.AddToViewport` _returnvalue 0)))

(fn `CheckWinCondition`
  (bind _value (`/Game/LoopHero/BP_GI_LoopHero.GetFlag` (`self.GameInstance`) "NewEnumerator6"))
  (if _value
    (bind _returnvalue (`|CreateWidget` "/Game/LoopHero/UI/WBP_WinScreen.WBP_WinScreen_C"))
    (`UserWidget.AddToViewport` _returnvalue 0)))

(fn `UserConstructionScript`)