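; Witness actor for the LoopHero game that opens dialogue matching the player's story progress.
; On BeginPlay it caches the LoopHero game instance and the level's dialogue manager, and stores the dialogue table.
; OpenDialogue tests game instance flags in a fixed priority chain and starts the first matching dialogue by ID through the manager, falling back to the intro dialogue when no flag is set.
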(event `self.ReceiveBeginPlay`
  (`|ExecutionSequence`
    (:`then_0`
      (bind _asbp_gi_loop_hero (cast `/Game/LoopHero/BP_GI_LoopHero` (`GameplayStatics.GetGameInstance`)))
      (set `self.GameInstance` _asbp_gi_loop_hero))
    (:`then_1`
      (bind _returnvalue (`GameplayStatics.GetActorOfClass` "/Game/LoopHero/BP_DialogueManager.BP_DialogueManager_C"))
      (set `self.DialogueManager` _returnvalue)
      (set `self.DialogueTable` "/Game/LoopHero/Data/DT_Dialogue.DT_Dialogue"))))

(fn `OpenDialogue`
  (bind _gameinstance (`self.GameInstance`))
  (bind _value (`/Game/LoopHero/BP_GI_LoopHero.GetFlag` _gameinstance "NewEnumerator6"))
  (if _value
    (`/Game/LoopHero/BP_DialogueManager.StartDialogue` (`self.DialogueManager`) "temoin_final")
    (return)
    (else
      (bind _value_2 (`/Game/LoopHero/BP_GI_LoopHero.GetFlag` _gameinstance "NewEnumerator3"))
      (if _value_2
        (`/Game/LoopHero/BP_DialogueManager.StartDialogue` (`self.DialogueManager`) "temoin_choix")
        (return)
        (else
          (bind _value_3 (`/Game/LoopHero/BP_GI_LoopHero.GetFlag` _gameinstance "NewEnumerator2"))
          (if _value_3
            (`/Game/LoopHero/BP_DialogueManager.StartDialogue` (`self.DialogueManager`) "temoin_relique")
            (return)
            (else
              (bind _value_4 (`/Game/LoopHero/BP_GI_LoopHero.GetFlag` _gameinstance "NewEnumerator1"))
              (if _value_4
                (`/Game/LoopHero/BP_DialogueManager.StartDialogue` (`self.DialogueManager`) "temoin_ruines")
                (return)
                (else
                  (`/Game/LoopHero/BP_DialogueManager.StartDialogue` (`self.DialogueManager`) "temoin_debut")
                  (return))))))))))

(fn `UserConstructionScript`)