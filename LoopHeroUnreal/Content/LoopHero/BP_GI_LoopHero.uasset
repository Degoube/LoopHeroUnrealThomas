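; Game instance for LoopHero that holds the narrative state: named flags, a loop counter and a resource amount.
; Defining a flag saves the state to a BP_SG_Narrative slot, while resource changes are bounds-checked but not saved.
; LoadProgress initializes state without a save; otherwise it writes current state into the loaded object, never restoring it.
; Resource updates rebuild the struct with the loop counter at zero.
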(fn `AddRessources`
  (params (Amount :type Integer))
  (set `self.NarrativeState` (make `/Game/LoopHero/Structure/S_NarrativeState` _ 0 (`KismetMathLibrary.Clamp` (+ Amount (`.Ressource_12_FAA554DE40ACD25208AABE834CBD9416` (break `/Game/LoopHero/Structure/S_NarrativeState` (`self.NarrativeState`)))) 0 999))))

(fn `DefineFlag`
  (params (Flag :type "/Game/LoopHero/Enumeration/E_NarrativeFlag Enum" :default "NewEnumerator0") (Value :type Boolean))
  (`BlueprintMapLibrary.Map_Add` (`.Flags_4_3309358B40C3436190912A91987CFC9B` (break `/Game/LoopHero/Structure/S_NarrativeState` (`self.NarrativeState`))) Flag Value)
  (`self.SaveProgress`)
  (return))

(fn `GetFlag`
  (params (Flag :type "/Game/LoopHero/Enumeration/E_NarrativeFlag Enum" :default "NewEnumerator0"))
  (returns (Value :type Boolean))
  (bind _flags (break `/Game/LoopHero/Structure/S_NarrativeState` (`self.NarrativeState`)))
  (if (`BlueprintMapLibrary.Map_Contains` _flags Flag)
    (return (`BlueprintMapLibrary.Map_Find` _flags (`local.Flag`)))
    (else
      (return false))))

(fn `InitializeState`
  (`BlueprintMapLibrary.Map_Clear` (`.Flags_4_3309358B40C3436190912A91987CFC9B` (break `/Game/LoopHero/Structure/S_NarrativeState` (`self.NarrativeState`))))
  (set `self.NarrativeState` (make `/Game/LoopHero/Structure/S_NarrativeState` _))
  (return))

(fn `LoadProgress`
  (returns (Sucess :type Boolean))
  (bind (_flags _loopcounter _ressource) (break `/Game/LoopHero/Structure/S_NarrativeState` (`self.NarrativeState`)))
  (bind _returnvalue (`GameplayStatics.DoesSaveGameExist` (`self.SaveName`)))
  (if _returnvalue
    (bind _returnvalue_2 (`GameplayStatics.LoadGameFromSlot` (`self.SaveName`)))
    (bind _asbp_sg_narrative (cast `/Game/LoopHero/BP_SG_Narrative` _returnvalue_2))
    (set `/Game/LoopHero/BP_SG_Narrative.Flags` _flags _asbp_sg_narrative)
    (set `/Game/LoopHero/BP_SG_Narrative.LoopCounter` _loopcounter _asbp_sg_narrative)
    (set `/Game/LoopHero/BP_SG_Narrative.Ressource` _ressource _asbp_sg_narrative)
    (return true)
    (else
      (`self.InitializeState`)
      (return false))))

(fn `RemoveResources`
  (params (Amount :type Integer))
  (returns (Sucess :type Boolean))
  (bind (_flags _loopcounter _ressource) (break `/Game/LoopHero/Structure/S_NarrativeState` (`self.NarrativeState`)))
  (if (>= _ressource Amount)
    (set `self.NarrativeState` (make `/Game/LoopHero/Structure/S_NarrativeState` _ 0 (- _ressource Amount)))
    (return true)
    (else
      (return false))))

(fn `SaveProgress`
  (bind (_flags _loopcounter _ressource) (break `/Game/LoopHero/Structure/S_NarrativeState` (`self.NarrativeState`)))
  (bind _returnvalue (`GameplayStatics.CreateSaveGameObject` "/Game/LoopHero/BP_SG_Narrative.BP_SG_Narrative_C"))
  (set `/Game/LoopHero/BP_SG_Narrative.Flags` _flags _returnvalue)
  (set `/Game/LoopHero/BP_SG_Narrative.LoopCounter` _loopcounter _returnvalue)
  (set `/Game/LoopHero/BP_SG_Narrative.Ressource` _ressource _returnvalue)
  (`GameplayStatics.SaveGameToSlot` _returnvalue (`self.SaveName`)))