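; Dialogue manager for LoopHero that plays branching conversations from the DT_Dialogue data table.
; StartDialogue looks up a node by ID, shows it only if its required GameInstance flags are set, then applies the flags it defines.
; ShowNode creates or reuses the dialogue box, showing either a continue button or choices.
; Continue and ChooseOption follow next-node IDs, with choices setting flags, and remove the box when none remains.
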(event `self.ReceiveBeginPlay`
  (`|ExecutionSequence`
    (:`then_0`
      (bind _asbp_gi_loop_hero (cast `/Game/LoopHero/BP_GI_LoopHero` (`GameplayStatics.GetGameInstance`)))
      (set `self.GameInstance` _asbp_gi_loop_hero))
    (:`then_1`
      (set `self.DialogueTable` "/Game/LoopHero/Data/DT_Dialogue.DT_Dialogue"))))

(fn `ApplyFlag`
  (params (Flag :type "Array of /Game/LoopHero/Enumeration/E_NarrativeFlag Enum"))
  (for _array_element Flag
    (`/Game/LoopHero/BP_GI_LoopHero.DefineFlag` (`self.GameInstance`) _array_element true))
  (return))

(fn `CheckFlag`
  (params (Node :type "/Game/LoopHero/Structure/S_DialoguesNodes Structure"))
  (returns (Valid :type Boolean))
  (bind (_nodeid _text _flagrequired) (break `/Game/LoopHero/Structure/S_DialoguesNodes` Node))
  (if (== (`KismetArrayLibrary.Array_Length` _flagrequired) 0)
    (return true)
    (else
      (for _array_element _flagrequired
        (bind _value (`/Game/LoopHero/BP_GI_LoopHero.GetFlag` (`self.GameInstance`) _array_element))
        (if (not _value)
          (return false)))
      (return true))))

(fn `ChooseOption`
  (params (ChoiceIndex :type Integer))
  (bind (_textchoice _flagstodefined _destinationidnode) (break `/Game/LoopHero/Structure/S_DialoguesChoice` (`|GetArrayItem` (`.Choice_18_B9AAC67D40EAF27761E2AB93061D6112` (break `/Game/LoopHero/Structure/S_DialoguesNodes` (`self.CurrentNode`))) ChoiceIndex)))
  (`self.ApplyFlag` (`|MakeArray` _flagstodefined))
  (if (`KismetStringLibrary.IsEmpty` _destinationidnode)
    (`Widget.RemoveFromParent` (`self.WidgetDialogue`))
    (set `self.WidgetDialogue` null)
    (else
      (`self.StartDialogue` _destinationidnode))))

(fn `Continue`
  (bind (_nodeid _text _flagrequired _flagtodefined _choice _nextnodeid) (break `/Game/LoopHero/Structure/S_DialoguesNodes` (`self.CurrentNode`)))
  (if (`KismetStringLibrary.IsEmpty` _nextnodeid)
    (`Widget.RemoveFromParent` (`self.WidgetDialogue`))
    (set `self.WidgetDialogue` null)
    (else
      (`self.StartDialogue` _nextnodeid))))

(fn `ShowNode`
  (bind _returnvalue (`GameplayStatics.GetPlayerController` 0))
  (bind _widgetdialogue (`self.WidgetDialogue`))
  (bind (_nodeid _text _flagrequired _flagtodefined _choice) (break `/Game/LoopHero/Structure/S_DialoguesNodes` (`self.CurrentNode`)))
  (if (`KismetSystemLibrary.IsValid` (`self.WidgetDialogue`))
    (`Widget.SetVisibility` (`self.WidgetDialogue`) "Visible")
    (elif (`KismetSystemLibrary.IsValid` _returnvalue)
      (bind _returnvalue_2 (`|CreateWidget` "/Game/LoopHero/UI/WBP_DialogueBox.WBP_DialogueBox_C" _returnvalue))
      (bind _output_get (set `self.WidgetDialogue` _returnvalue_2))
      (`UserWidget.AddToViewport` _returnvalue_2 10)
      (`UserWidget.AddToViewport` _output_get 10)
      (`WidgetBlueprintLibrary.SetInputMode_UIOnlyEx` null _output_get)
      (set `PlayerController.bShowMouseCursor` true _returnvalue)
      (else
        (return))))
  (`/Game/LoopHero/UI/WBP_DialogueBox.ShowText` _widgetdialogue _text)
  (if (== (`KismetArrayLibrary.Array_Length` _choice) 0)
    (`/Game/LoopHero/UI/WBP_DialogueBox.ShowContinueButton` _widgetdialogue)
    (else
      (`/Game/LoopHero/UI/WBP_DialogueBox.ShowChoice` _widgetdialogue _choice))))

(fn `StartDialogue`
  (params (NodeId :type String))
  (bind _returnvalue (`|GetDataTableRow` (`self.DialogueTable`) (`KismetStringLibrary.Conv_StringToName` NodeId))
    (:`then`
      (bind _valid (`self.CheckFlag` _returnvalue))
      (if _valid
        (bind _output_get (set `self.CurrentNode` _returnvalue))
        (`self.ApplyFlag` (`.FlagToDefined_11_7FE68A264F67B706005B3A925740998A` (break `/Game/LoopHero/Structure/S_DialoguesNodes` _output_get)))
        (`self.ShowNode`)))))

(fn `UserConstructionScript`)