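; BP_Pawn is a board game pawn that moves between numbered cells on a Board.
; Its current cell number lives in BP_LoopGameInstance; BeginPlay snaps the pawn to that cell and creates the dialogue UI, handing it the Dice and itself.
; TryMoving asks the Board for the destination cell, saves it, teleports the pawn there and activates it.
; ActivateCell and UpdateCell forward message calls to the current cell.
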(event `self.ReceiveBeginPlay`
  (bind _asbp_loop_game_instance (cast `/Game/Blueprints/Global/BP_LoopGameInstance` (`GameplayStatics.GetGameInstance`)))
  (set `self.BP Loop Game Instance` _asbp_loop_game_instance)
  (`self.MoveToCell`)
  (bind _returnvalue (`|CreateWidget` "/Game/Blueprints/Global/WBP_DialogueUI.WBP_DialogueUI_C"))
  (bind _output_get (set `self.Widget` _returnvalue))
  (set `/Game/Blueprints/Global/WBP_DialogueUI.Dice` (`self.Dice`) _output_get)
  (set `/Game/Blueprints/Global/WBP_DialogueUI.Pawn` self _output_get)
  (`UserWidget.AddToViewport` _output_get 0))

(fn `ActivateCell`
  (bind _cell (`/Game/Blueprints/Gameplay/BP_Board.GetCellByNumber` (`self.Board`) (`/Game/Blueprints/Global/BP_LoopGameInstance. CellNumber` (`self.BP Loop Game Instance`))))
  (message `/Game/Blueprints/Gameplay/BPI_Activable.Activate` _cell self))

(fn `MoveToCell`
  (bind _cell (`/Game/Blueprints/Gameplay/BP_Board.GetCellByNumber` (`self.Board`) (`/Game/Blueprints/Global/BP_LoopGameInstance. CellNumber` (`self.BP Loop Game Instance`))))
  (bind (_returnvalue_location _returnvalue_rotation) (`KismetMathLibrary.BreakTransform` (`self.GetTransform` _cell)))
  (`self.K2_SetActorLocation` _returnvalue_location)
  (`self.K2_SetActorRotation` _returnvalue_rotation))

(fn `TryMoving`
  (params (Value :type Integer))
  (bind _bp_loop_game_instance (`self.BP Loop Game Instance`))
  (bind _cell (`/Game/Blueprints/Gameplay/BP_Board.GetNextCellToMove` (`self.Board`) (+ Value (`/Game/Blueprints/Global/BP_LoopGameInstance. CellNumber` _bp_loop_game_instance))))
  (set `/Game/Blueprints/Global/BP_LoopGameInstance. CellNumber` _cell _bp_loop_game_instance)
  (`self.MoveToCell`)
  (`self.ActivateCell`))

(fn `UpdateCell`
  (bind _cell (`/Game/Blueprints/Gameplay/BP_Board.GetCellByNumber` (`self.Board`) (`/Game/Blueprints/Global/BP_LoopGameInstance. CellNumber` (`self.BP Loop Game Instance`))))
  (message `/Game/Blueprints/Gameplay/BPI_Activable.Update` _cell self))

(fn `UserConstructionScript`)