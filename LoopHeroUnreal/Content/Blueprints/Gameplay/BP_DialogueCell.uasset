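; BP_DialogueCell is an actor that feeds row-based dialogue to the interacting pawn's widget.
; Activate reads the current row from its BPCDialogueComponent, sends the character and long dialogue text to the widget, then starts the dialogue.
; Update either exits the widget when the dialogue is finished or advances to the next row and refreshes the displayed character and text.
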(event `/Game/Blueprints/Gameplay/BPI_Activable.Activate`
  (params (Pawn :type "/Game/Blueprints/Gameplay/BP_Pawn Object Reference"))
  (bind _bpc_dialoguecomponent (`self.BPC_DialogueComponent`))
  (bind _widget (`/Game/Blueprints/Gameplay/BP_Pawn.Widget` Pawn))
  (`/Game/Blueprints/Global/BPC_DialogueComponent.GetCurrentDialogueRowData` _bpc_dialoguecomponent)
  (bind _charactername (`/Game/Blueprints/Global/BPC_DialogueComponent.GetCharacterFromCurrentRow` _bpc_dialoguecomponent))
  (bind _dialoguelong (`/Game/Blueprints/Global/BPC_DialogueComponent.GetDialogueLongFromCurrentRow` _bpc_dialoguecomponent))
  (`/Game/Blueprints/Global/WBP_DialogueUI.UpdateDialogue` _widget _charactername _dialoguelong)
  (`/Game/Blueprints/Global/WBP_DialogueUI.StartDialogue` _widget))

(event `/Game/Blueprints/Gameplay/BPI_Activable.Update`
  (params (Pawn :type "/Game/Blueprints/Gameplay/BP_Pawn Object Reference"))
  (bind _bpc_dialoguecomponent (`self.BPC_DialogueComponent`))
  (bind _widget (`/Game/Blueprints/Gameplay/BP_Pawn.Widget` Pawn))
  (bind _bisfinished (`/Game/Blueprints/Global/BPC_DialogueComponent.IsDialogueFinished` _bpc_dialoguecomponent))
  (if _bisfinished
    (`/Game/Blueprints/Global/WBP_DialogueUI.ExitDialogue` _widget)
    (else
      (`/Game/Blueprints/Global/BPC_DialogueComponent.ReadNextRow` _bpc_dialoguecomponent)
      (bind _charactername (`/Game/Blueprints/Global/BPC_DialogueComponent.GetCharacterFromCurrentRow` _bpc_dialoguecomponent))
      (bind _dialoguelong (`/Game/Blueprints/Global/BPC_DialogueComponent.GetDialogueLongFromCurrentRow` _bpc_dialoguecomponent))
      (`/Game/Blueprints/Global/WBP_DialogueUI.UpdateDialogue` _widget _charactername _dialoguelong))))

(fn `UserConstructionScript`
  (`parent.UserConstructionScript`))